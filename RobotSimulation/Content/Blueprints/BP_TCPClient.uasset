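; BP_TCPClient is an actor that acts as a TCP client to a server on localhost port 8000.
; It connects on BeginPlay, stores the connection ID, and disconnects on EndPlay if still connected.
; Callbacks print connect and disconnect notices, and pass each received message to ParseJSONFromTCP, which is defined outside these graphs, before printing it as a string.
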(event Custom|Disconnected
  (params (ConnectionId :type Integer))
  (Development|PrintString "Disconnected" true true "(R=0.000000,G=0.660000,B=1.000000,A=1.000000)" 15.0))

(event Custom|ConnectionEstablished
  (params (ConnectionId :type Integer))
  (Development|PrintString "Client : Connected" true true "(R=0.000000,G=0.660000,B=1.000000,A=1.000000)" 5.0))

(event Custom|Received
  (params (ConnectionId :type Integer) (Message :type Array%20of%20Bytes))
  (Class|TCPClient|ParseJSONfromTCP Message)
  (bind _returnvalue (Class|TcpSocketConnection|MessageReadString Message))
  (Development|PrintString _returnvalue))

(event EventBeginPlay
  (bind _connectionid (Class|TcpSocketConnection|Connect "127.0.0.1" 8000 (delegate Custom|Disconnected) (delegate Custom|ConnectionEstablished) (delegate Custom|Received)))
  (Variables|Default|SetConnection%20Id _connectionid))

(event Collision|EventActorBeginOverlap
  (params (OtherActor :type Actor%20Object%20Reference)))

(event EventTick
  (params (DeltaSeconds :type Float%20%28single-precision%29)))

(event EventEndPlay
  (params (EndPlayReason :type EEndPlayReason%20Enum :default "Destroyed"))
  (if (Class|TcpSocketConnection|IsConnected (Variables|Default|GetConnection%20Id))
    (Class|TcpSocketConnection|Disconnect (Variables|Default|GetConnection%20Id))))

(fn ConstructionScript)