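; Test actor that acts as a socket client, connecting to a server on the local machine at BeginPlay and storing the connection ID.
; On connection it sends a test string converted to bytes.
; Connect, disconnect and message callbacks print to screen, with incoming messages decoded as strings using the full message length.
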(event Custom|Connected
  (params (ConnectionId :type Integer))
  (Development|PrintString "Client : Connected" true true "(R=0.000000,G=0.660000,B=1.000000,A=1.000000)" 5.0)
  (Class|TcpSocketConnection|SendData (Variables|Default|GetConnection%20Id) (Class|TcpSocketConnection|ToBytes(String) "Testing msg from unreal Engine")))

(event Custom|Msg
  (params (ConnectionId :type Integer) (Message :type Array%20of%20Bytes))
  (bind _returnvalue (Class|TcpSocketConnection|MessageReadString Message (Utilities|Array|Length Message)))
  (Development|PrintString (Utilities|String|Append "Client : Recieved : " _returnvalue)))

(event Custom|Disconned
  (params (ConnectionId :type Integer))
  (Development|PrintString "Client : Disconnected" true true "(R=0.000000,G=0.660000,B=1.000000,A=1.000000)" 5.0))

(event EventBeginPlay
  (bind _connectionid (Class|TcpSocketConnection|Connect "127.0.0.1" 8000 (delegate Custom|Disconned) (delegate Custom|Connected) (delegate Custom|Msg)))
  (Variables|Default|SetConnection%20Id _connectionid))

(event Collision|EventActorBeginOverlap
  (params (OtherActor :type Actor%20Object%20Reference)))

(event EventTick
  (params (DeltaSeconds :type Float%20%28single-precision%29)))

(event Input|KeyboardEvents|SpaceBar
  (params (Key :type Key%20Structure)))

(fn ConstructionScript)